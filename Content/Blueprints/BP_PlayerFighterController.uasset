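; Player controller for a fighting game that turns Enhanced Input actions into fighter combat moves and steps.
; On BeginPlay it adds the in-game mapping context.
; Jab, cross and rear kick inputs queue straight punches and kicks into the CombatController's action buffer, while dash right plays a step montage directly on player 0's mesh.
; A helper returns the controlled pawn cast to Fighter.
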(event `self.ReceiveBeginPlay`
  (`EnhancedInputSubsystemInterface.AddMappingContext` (subsystem `EnhancedInputLocalPlayerSubsystem`) "/Game/Input/InputMappings/IM_InGame.IM_InGame" 0 (struct)))

(event `EnhancedInput|/Game/Input/InputActions/IA_Cross`
  (params (ActionValue :type Boolean) (ElapsedSeconds :type "Float (double-precision)") (TriggeredSeconds :type "Float (double-precision)") (InputAction :type "InputAction Object Reference" :default "/Game/Input/InputActions/IA_Cross.IA_Cross"))
  (:`Completed`
    (`CombatControllerComponent.AddToCombatActionBuffer` (`self.CombatController`) "Rear_Straight")))

(event `EnhancedInput|/Game/Input/InputActions/IA_RearKick`
  (params (ActionValue :type Boolean) (ElapsedSeconds :type "Float (double-precision)") (TriggeredSeconds :type "Float (double-precision)") (InputAction :type "InputAction Object Reference" :default "/Game/Input/InputActions/IA_RearKick.IA_RearKick"))
  (:`Completed`
    (`CombatControllerComponent.AddToCombatActionBuffer` (`self.CombatController`) "Rear_Kick")))

(event `EnhancedInput|/Game/Input/InputActions/IA_Jab`
  (params (ActionValue :type Boolean) (ElapsedSeconds :type "Float (double-precision)") (TriggeredSeconds :type "Float (double-precision)") (InputAction :type "InputAction Object Reference" :default "/Game/Input/InputActions/IA_Jab.IA_Jab"))
  (:`Completed`
    (`CombatControllerComponent.AddToCombatActionBuffer` (`self.CombatController`) "Lead_Straight")))

(event `EnhancedInput|/Game/Input/InputActions/IA_DashRight`
  (params (ActionValue :type Boolean) (ElapsedSeconds :type "Float (double-precision)") (TriggeredSeconds :type "Float (double-precision)") (InputAction :type "InputAction Object Reference" :default "/Game/Input/InputActions/IA_DashRight.IA_DashRight"))
  ;[1 1 1] Movement
  (:`Completed`
    (`|PlayMontage` (`Character.Mesh` (`GameplayStatics.GetPlayerCharacter` 0)) "/Game/Characters/Mannequins/Animations/Manny/Movement/AM_MediumStepRight.AM_MediumStepRight")))

(fn `GetPossessedFighter`
  (returns (`Possessed Fighter` :type "Fighter Object Reference"))
  (bind _asfighter (cast `Fighter` (`self.K2_GetPawn` self))
    (:`then`
      (return _asfighter))
    (:`CastFailed`
      (return null))))

(fn `UserConstructionScript`)