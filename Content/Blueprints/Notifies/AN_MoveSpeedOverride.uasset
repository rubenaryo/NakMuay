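; Anim notify state that overrides a Fighter's max movement speed for the span of an animation.
; On begin it casts the mesh owner to Fighter and its movement to FighterMovementComponent, then sets the override to the MoveSpeedOverride value.
; On end it resets that override through the same casts, returning false in either event if a cast fails.
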(fn `Received_NotifyBegin`
  (params (MeshComp :type "SkeletalMeshComponent Object Reference") (Animation :type "AnimSequenceBase Object Reference") (TotalDuration :type "Float (single-precision)") (EventReference :type "AnimNotifyEventReference Structure (by ref)"))
  (returns (ReturnValue :type Boolean))
  (bind _asfighter (cast `Fighter` (`ActorComponent.GetOwner` MeshComp))
    (:`then`
      (bind _asfighter_movement_component (cast `FighterMovementComponent` (`Character.CharacterMovement` _asfighter))
        (:`then`
          (`FighterMovementComponent.SetOverrideMaxSpeed` _asfighter_movement_component (`self.MoveSpeedOverride`))
          (return true))
        (:`CastFailed`
          _)))
    (:`CastFailed`
      _))
  (return false))

(fn `Received_NotifyEnd`
  (params (MeshComp :type "SkeletalMeshComponent Object Reference") (Animation :type "AnimSequenceBase Object Reference") (EventReference :type "AnimNotifyEventReference Structure (by ref)"))
  (returns (ReturnValue :type Boolean))
  (bind _asfighter (cast `Fighter` (`ActorComponent.GetOwner` MeshComp))
    (:`then`
      (bind _asfighter_movement_component (cast `FighterMovementComponent` (`Character.CharacterMovement` _asfighter))
        (:`then`
          (`FighterMovementComponent.ResetOverrideMaxSpeed` _asfighter_movement_component)
          (return true))
        (:`CastFailed`
          _)))
    (:`CastFailed`
      _))
  (return false))