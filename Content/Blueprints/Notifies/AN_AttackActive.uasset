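; Anim notify state that marks the active hit window of an attack animation on a Fighter.
; Begin, tick and end each cast the mesh owner to Fighter and forward to its CombatComponent's active-attack handlers.
; It passes its collider area and physics hit strength to all three, adding trace radius and local push impulse on tick, so the component handles the hit logic.
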(fn `Received_NotifyBegin`
  (params (MeshComp :type "SkeletalMeshComponent Object Reference") (Animation :type "AnimSequenceBase Object Reference") (TotalDuration :type "Float (single-precision)") (EventReference :type "AnimNotifyEventReference Structure (by ref)"))
  (returns (ReturnValue :type Boolean))
  (bind _asfighter (cast `Fighter` (`ActorComponent.GetOwner` MeshComp))
    (:`then`
      (`/Engine/EditorBlueprintResources/StandardMacros.IsValid` _asfighter
        (:`Is Valid`
          (`CombatActorComponent.HandleActiveAttackBegin` (`Fighter.CombatComponent` _asfighter) (`self.Collider Area`) (`self.PhysicsHitStrength`))
          (return true))
        (:`Is Not Valid`
          _)))
    (:`CastFailed`
      _))
  (return false))

(fn `Received_NotifyEnd`
  (params (MeshComp :type "SkeletalMeshComponent Object Reference") (Animation :type "AnimSequenceBase Object Reference") (EventReference :type "AnimNotifyEventReference Structure (by ref)"))
  (returns (ReturnValue :type Boolean))
  (bind _asfighter (cast `Fighter` (`ActorComponent.GetOwner` MeshComp)))
  (`CombatActorComponent.HandleActiveAttackEnd` (`Fighter.CombatComponent` _asfighter) (`self.Collider Area`) (`self.PhysicsHitStrength`))
  (return true))

(fn `Received_NotifyTick`
  (params (MeshComp :type "SkeletalMeshComponent Object Reference") (Animation :type "AnimSequenceBase Object Reference") (FrameDeltaTime :type "Float (single-precision)") (EventReference :type "AnimNotifyEventReference Structure (by ref)"))
  (returns (ReturnValue :type Boolean))
  (bind _asfighter (cast `Fighter` (`ActorComponent.GetOwner` MeshComp)))
  (`CombatActorComponent.HandleActiveAttackTick` (`Fighter.CombatComponent` _asfighter) (`self.Collider Area`) (`self.Trace Radius`) (`self.PhysicsHitStrength`) (`self.Local Push Impulse`))
  (return true))