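; Physical animation component on a Fighter that plays physics-driven hit reactions on its skeletal mesh.
; On a hit, it queues a job, simulates bodies below the struck bone, applies physical animation and constraint profiles from the training GameMode per attack type, and adds an impulse along the trace.
; Tick eases each active hit's physics blend weight to zero.
; FinalizeHit is empty, so simulation stays enabled; debug text and arrows remain.
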(event `self.ReceiveBeginPlay`
  (`parent.ReceiveBeginPlay`)
  (bind _asfighter (cast `Fighter` (`self.GetOwner`)))
  (bind _returnvalue (`Actor.GetComponentByClass` _asfighter "/Script/Engine.SkeletalMeshComponent"))
  (set `self.Mesh` _returnvalue)
  (`self.SetSkeletalMeshComponent` _returnvalue))

(fn `FinalizeHit`
  (return))

(fn `GetHitProfileFromCombatActionType`
  (params (`Combat Action Type` :type "ECombatActionType Enum" :default "None"))
  (returns (HitProfileName :type Name))
  (bind _asbp_fight_training_game_mode (cast `/Game/Blueprints/BP_FightTrainingGameMode` (`GameplayStatics.GetGameMode`)))
  (if (`KismetSystemLibrary.IsValid` _asbp_fight_training_game_mode)
    (return (`FightTrainingGameMode.GetHitProfileFromCombatAction` _asbp_fight_training_game_mode `Combat Action Type`))
    (else
      (return "None"))))

(fn `InitiateHit`
  (params (Impulse :type "Vector Structure (by ref)") (`Impact Point` :type "Vector Structure") (`Hit Bone Name` :type Name) (`Attack Type` :type "ECombatActionType Enum" :default "None"))
  (returns (`Valid Hit` :type Boolean))
  (locals (LocalHitBoneName :type Name :default "None") (LocalImpulse :type "Vector Structure"))
  (bind _localimpulse (`local.LocalImpulse`))
  (bind _localhitbonename (`local.LocalHitBoneName`))
  (set `local.LocalHitBoneName` `Hit Bone Name`)
  (set `local.LocalImpulse` Impulse)
  (bind _valid (`self.Is Hit Valid` Impulse `Impact Point` `Hit Bone Name`))
  (if _valid
    (`self.PushActiveHit` (make `HitReactionJob` Impulse `Impact Point` `Hit Bone Name`))
    (`self.SetComponentTickEnabled` true)
    (`SkeletalMeshComponent.SetAllBodiesBelowSimulatePhysics` (`self.Mesh`) (`local.LocalHitBoneName`) true true)
    (bind _hitprofilename (`self.GetHitProfileFromCombatActionType` `Attack Type`))
    (`self.ApplyPhysicalAnimationProfileBelow` (`local.LocalHitBoneName`) _hitprofilename)
    (`SkeletalMeshComponent.SetConstraintProfileForAll` (`self.Mesh`) _hitprofilename false)
    (`SkeletalMeshComponent.AccumulateAllBodiesBelowPhysicsBlendWeight` (`self.Mesh`) (`local.LocalHitBoneName`) 1.0 false)
    (`PrimitiveComponent.AddImpulse` (`self.Mesh`) _localimpulse _localhitbonename true)
    (`KismetSystemLibrary.PrintText` (`|FormatText` "{0} {1}" (`KismetTextLibrary.Conv_VectorToText` _localimpulse) _localhitbonename) true false)
    (return true)
    (else
      (return false))))

(fn `Is Hit Valid`
  (params (Impulse :type "Vector Structure (by ref)") (`Impact Point` :type "Vector Structure (by ref)") (`Hit Bone Name` :type "Name (by ref)"))
  (returns (Valid :type Boolean))
  (return (and (!= (`KismetMathLibrary.VSizeSquared` Impulse) 0.0) (!= `Hit Bone Name` "None"))))

(fn `IsBlending`
  (params (BlendWeight :type "Float (double-precision)"))
  (returns (Blending :type Boolean))
  (return (> BlendWeight 0.001)))

(fn `OnGetHit_Implementation`
  (params (HitComp :type "PrimitiveComponent Object Reference") (AttackingFighter :type "Fighter Object Reference") (InHitResult :type "HitResult Structure (by ref)") (AttackType :type "ECombatActionType Enum" :default "None") (PhysicsHitStrength :type "Float (single-precision)"))
  (returns (ReturnValue :type Boolean))
  (bind (_bblockinghit _binitialoverlap _time _distance _location _impactpoint _normal _impactnormal _physmat _hitactor _hitcomponent _hitbonename _bonename _hititem _elementindex _faceindex _tracestart _traceend) (`GameplayStatics.BreakHitResult` InHitResult))
  (bind _returnvalue (`SceneComponent.GetSocketLocation` (`self.Mesh`) _hitbonename))
  (bind _returnvalue_2 (* (`KismetMathLibrary.Normal` (- _traceend _tracestart)) PhysicsHitStrength))
  (bind _valid_hit (`self.InitiateHit` _returnvalue_2 _impactpoint _hitbonename AttackType))
  (if _valid_hit
    (`KismetSystemLibrary.DrawDebugArrow` _returnvalue (+ _returnvalue _returnvalue_2) 10.0 (struct :`R` 1.0 :`G` 0.09 :`B` 0.969463 :`A` 1.0) 1.0 3.0))
  (return _valid_hit))

(fn `Tick_Implementation`
  (params (DeltaTime :type "Float (single-precision)"))
  (locals (`Prev Blend Weight` :type "Float (double-precision)" :default 0.0) (LocalHitBoneName :type Name))
  (`self.TickActiveHits` DeltaTime)
  (return))

(fn `TickSingleActiveHit_Implementation`
  (params (DeltaTime :type "Float (single-precision)") (InHitReactionRef :type "HitReactionJob Structure (by ref)"))
  (returns (ReturnValue :type Boolean))
  (locals (`Local Hit Bone Name` :type Name :default "None") (`Prev Blend Weight` :type "Float (double-precision)" :default 0.0) (`New Blend Weight` :type "Float (double-precision)" :default 0.0))
  (bind (_hitimpulse _impactpoint _hitbonename _blendweight) (break `HitReactionJob` InHitReactionRef))
  (bind _blending (`self.IsBlending` _blendweight))
  (if _blending
    (set `local.Local Hit Bone Name` _hitbonename)
    (bind _output_get (set `local.Prev Blend Weight` _blendweight))
    (bind _output_get_2 (set `local.New Blend Weight` (`KismetMathLibrary.FInterpTo` _output_get 0.0 DeltaTime 4.0)))
    (`self.SetActiveHitBlendWeight` InHitReactionRef _output_get_2)
    (`SkeletalMeshComponent.SetAllBodiesBelowPhysicsBlendWeight` (`self.Mesh`) (`local.Local Hit Bone Name`) (`local.New Blend Weight`) false true)
    (bind _blending_2 (`self.IsBlending` (`local.New Blend Weight`)))
    (if (not _blending_2)
      (`self.FinalizeHit`)
      (return true)
      (else
        (return false)))
    (else
      (return false))))