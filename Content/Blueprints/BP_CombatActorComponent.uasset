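; BP_CombatActorComponent is a combat component that turns queued combat actions into animation montages on a skeletal mesh.
; Each tick, when an action can be consumed, it takes the next one from the queue and looks up its montage through BP_FightTrainingGameMode.
; It plays the montage, records the current action type, and resets combat state when playback completes.
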(event `self.ReceiveTick`
  (params (DeltaSeconds :type "Float (single-precision)"))
  (bind _returnvalue (`self.AbleToConsumeAction`))
  (if _returnvalue
    (bind (_combatactiontype _returnvalue_2) (`self.GetNextCombatActionInQueue`))
    (if _returnvalue_2
      (bind _montage (`self.InternalGetAnimMontageFromCombatAction` _combatactiontype))
      (`|PlayMontage` (`self.GetSkeletalMeshComponent`) _montage
        (:`then`
          (`self.SetCurrentCombatActionType` _combatactiontype))
        (:`OnCompleted`
          (`self.ResetCombatState`))))))

(fn `InternalGetAnimMontageFromCombatAction`
  (params (`Combat Action Type` :type "ECombatActionType Enum" :default "None"))
  (returns (Montage :type "AnimMontage Object Reference"))
  (bind _asbp_fight_training_game_mode (cast `/Game/Blueprints/BP_FightTrainingGameMode` (`GameplayStatics.GetGameMode`)))
  (if (`KismetSystemLibrary.IsValid` _asbp_fight_training_game_mode)
    (bind _asanim_montage (cast `AnimMontage` (`FightTrainingGameMode.GetAnimMontageForCombatActionType` _asbp_fight_training_game_mode `Combat Action Type`)))
    (return _asanim_montage)))